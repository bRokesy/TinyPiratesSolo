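; Player controller that turns Enhanced Input into control of a BP_Ship and its main cannon.
; On BeginPlay it adds the IMC_Ship mapping context, and on possession it caches the ship and its main cannon.
; Throttle and turn actions set inputs on the ship, and aim toggles its aiming flag.
; Look steers the cannon only while aiming, and fire calls the cannon directly, both with debug prints.
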(event Input|EnhancedActionEvents|EnhancedInputActionIA_Look
  (params (ActionValue :type Vector%202D%20Structure) (ElapsedSeconds :type Float%20%28double-precision%29) (TriggeredSeconds :type Float%20%28double-precision%29) (InputAction :type Input%20Action%20Object%20Reference :default "/Game/Input/Action/IA_Look.IA_Look"))
  (bind (_x _y) (Math|Vector2D|BreakVector2D ActionValue))
  (:Triggered
    (if (Variables|/Game/Blueprints/BP_Ship.BP_Ship_C|GetbIsAiming (Variables|Default|GetControlledShip))
      (Default|AimCannon (Variables|Default|GetControlledCannon) _x _y)
      (Development|PrintString (Utilities|String|ToString(Float) _y) true false "(R=1.000000,G=0.010580,B=0.000000,A=1.000000)"))))

(event Input|EnhancedActionEvents|EnhancedInputActionIA_Throttle
  (params (ActionValue :type Float%20%28double-precision%29) (ElapsedSeconds :type Float%20%28double-precision%29) (TriggeredSeconds :type Float%20%28double-precision%29) (InputAction :type Input%20Action%20Object%20Reference :default "/Game/Input/Action/IA_Throttle.IA_Throttle"))
  (bind _controlledship (Variables|Default|GetControlledShip))
  (:Started
    (Variables|/Game/Blueprints/BP_Ship.BP_Ship_C|SetThrottleInput _controlledship ActionValue))
  (:Completed
    (Variables|/Game/Blueprints/BP_Ship.BP_Ship_C|SetThrottleInput _controlledship 0.0)))

(event Input|EnhancedActionEvents|EnhancedInputActionIA_Turn
  (params (ActionValue :type Float%20%28double-precision%29) (ElapsedSeconds :type Float%20%28double-precision%29) (TriggeredSeconds :type Float%20%28double-precision%29) (InputAction :type Input%20Action%20Object%20Reference :default "/Game/Input/Action/IA_Turn.IA_Turn"))
  (bind _controlledship (Variables|Default|GetControlledShip))
  (:Triggered
    (Variables|/Game/Blueprints/BP_Ship.BP_Ship_C|SetTurnInput _controlledship ActionValue))
  (:Completed
    (Variables|/Game/Blueprints/BP_Ship.BP_Ship_C|SetTurnInput _controlledship 0.0)))

(event Input|EnhancedActionEvents|EnhancedInputActionIA_Aim
  (params (ActionValue :type Boolean) (ElapsedSeconds :type Float%20%28double-precision%29) (TriggeredSeconds :type Float%20%28double-precision%29) (InputAction :type Input%20Action%20Object%20Reference :default "/Game/Input/Action/IA_Aim.IA_Aim"))
  (bind _controlledship (Variables|Default|GetControlledShip))
  (:Started
    (Variables|/Game/Blueprints/BP_Ship.BP_Ship_C|SetbIsAiming _controlledship true))
  (:Completed
    (Variables|/Game/Blueprints/BP_Ship.BP_Ship_C|SetbIsAiming _controlledship false)))

(event Input|EnhancedActionEvents|EnhancedInputActionIA_Fire
  (params (ActionValue :type Boolean) (ElapsedSeconds :type Float%20%28double-precision%29) (TriggeredSeconds :type Float%20%28double-precision%29) (InputAction :type Input%20Action%20Object%20Reference :default "/Game/Input/Action/IA_Fire.IA_Fire"))
  (:Triggered
    (Default|Fire (Variables|Default|GetControlledCannon))
    (Development|PrintString "Fire" true false "(R=1.000000,G=0.010580,B=0.000000,A=1.000000)")))

(event EventBeginPlay
  (bind _returnvalue (PlayerController|LocalPlayerSubsystems|GetEnhancedInputLocalPlayerSubsystem))
  (Utilities|IsValid _returnvalue
    (:Is%20Valid
      (Input|AddMappingContext _returnvalue "/Game/Input/IMC_Ship.IMC_Ship" 0 "(bIgnoreAllPressedKeysUntilRelease=True,bForceImmediately=False,bNotifyUserSettings=False)"))))

(event EventPossess
  (params (PossessedPawn :type Pawn%20Object%20Reference))
  (bind _asbp_ship (Utilities|Casting|CastToBP_Ship PossessedPawn))
  (bind _output_get (Variables|Default|SetControlledShip _asbp_ship))
  (bind _currentcannon (Default|GetMainCannon _output_get))
  (Variables|Default|SetControlledCannon _currentcannon))

(fn ConstructionScript)