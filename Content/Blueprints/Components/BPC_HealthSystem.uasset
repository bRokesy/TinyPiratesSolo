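; BPC_HealthSystem is an actor component that tracks its owner's health and destroys the owner when health reaches zero.
; On BeginPlay it adds a screen-space widget component above the owner and creates a WBP_HealthBar, though the graph never assigns that bar to the component.
; It binds to the owner's OnTakeAnyDamage, subtracting damage with clamping and updating the bar while health remains.
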(event Custom|OnDamageReceived
  (params (DamagedActor :type Actor%20Object%20Reference) (Damage :type Float%20%28single-precision%29) (DamageType :type Damage%20Type%20Object%20Reference) (InstigatedBy :type Controller%20Object%20Reference) (DamageCauser :type Actor%20Object%20Reference))
  (bind _maxhealth (Variables|Default|GetMaxHealth))
  (Variables|Default|SetHealth (Math|Float|Clamp(Float) (- (Variables|Default|GetHealth) Damage) 0.0 (Variables|Default|GetMaxHealth)))
  (if (<= (Variables|Default|GetHealth) 0.0)
    (Actor|DestroyActor (Components|GetOwner))
    (else
      (Default|UpdateHealth (Variables|Default|GetWidgetRef) (/ (Variables|Default|GetHealth) _maxhealth) (Variables|Default|GetHealth) _maxhealth))))

(event EventBeginPlay
  (bind _returnvalue (Game|AddComponentbyClass (Components|GetOwner) "/Script/UMG.WidgetComponent" true))
  (Class|WidgetComponent|SetWidgetSpace _returnvalue "Screen")
  (Class|WidgetComponent|SetDrawSize _returnvalue "(X=120.000000,Y=20.000000)")
  (Transformation|AttachComponentToComponent _returnvalue (Variables|/Script/Engine.Actor|GetRootComponent (Components|GetOwner)) "None" "KeepRelative" "KeepRelative" "KeepRelative" true)
  (Transformation|SetRelativeLocation _returnvalue "0.000000,0.000000,400.000000" false false)
  (bind _returnvalue_2 (UserInterface|CreateWidget "/Game/UI/Player/WBP_HealthBar.WBP_HealthBar_C"))
  (bind _output_get (Variables|Default|SetWidgetRef _returnvalue_2))
  (Default|UpdateHealth _output_get (/ (Variables|Default|GetHealth) (Variables|Default|GetMaxHealth)) (Variables|Default|GetHealth) (Variables|Default|GetMaxHealth))
  (EventDispatchers|BindEventtoOnTakeAnyDamage (Components|GetOwner) (delegate Custom|OnDamageReceived)))