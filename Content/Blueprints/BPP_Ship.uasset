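; Player-controlled ship pawn that moves with physics and fires an aimable cannon.
; Tick applies flattened forward force and turning torque, but only while throttle is positive and horizontal speed is below the maximum.
; Holding aim changes spring arm length and FOV, and lets look input set clamped rotations on the camera arm and cannon yaw/pitch pivots.
; Firing while aiming spawns a cannonball at the muzzle point.
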(event Input|EnhancedActionEvents|EnhancedInputActionIA_Aim
  (params (ActionValue :type Boolean) (ElapsedSeconds :type Float%20%28double-precision%29) (TriggeredSeconds :type Float%20%28double-precision%29) (InputAction :type Input%20Action%20Object%20Reference :default "/Game/Input/Action/IA_Aim.IA_Aim"))
  (:Triggered
    (Variables|/Script/Engine.SpringArmComponent|SetTargetArmLength (Variables|Default|GetSpringArm) (Variables|Aiming|GetAimCameraArmLength))
    (Camera|SetFieldOfView (Variables|Default|GetCamera) 75.0))
  (:Completed
    (Variables|/Script/Engine.SpringArmComponent|SetTargetArmLength (Variables|Default|GetSpringArm) (Variables|Aiming|GetNormalCameraArmLength))
    (Camera|SetFieldOfView (Variables|Default|GetCamera) 9e+01)))

(event Input|EnhancedActionEvents|EnhancedInputActionIA_Look
  (params (ActionValue :type Vector%202D%20Structure) (ElapsedSeconds :type Float%20%28double-precision%29) (TriggeredSeconds :type Float%20%28double-precision%29) (InputAction :type Input%20Action%20Object%20Reference :default "/Game/Input/Action/IA_Look.IA_Look"))
  (bind (_x _y) (Math|Vector2D|BreakVector2D ActionValue))
  (CallFunction|CannonRotation (Variables|Aiming|GetbIsAiming) _x _y (Variables|Aiming|GetAimSensitivity)))

(event Input|EnhancedActionEvents|EnhancedInputActionIA_Fire
  (params (ActionValue :type Boolean) (ElapsedSeconds :type Float%20%28double-precision%29) (TriggeredSeconds :type Float%20%28double-precision%29) (InputAction :type Input%20Action%20Object%20Reference :default "/Game/Input/Action/IA_Fire.IA_Fire"))
  (:Started
    (if (Variables|Aiming|GetbIsAiming)
      (CallFunction|Fire))))

(event EventTick
  (params (DeltaSeconds :type Float%20%28single-precision%29))
  (bind _ischecked (CallFunction|MovementCheck (Variables|Movement|GetThrottleInput) (Variables|Movement|GetMaxSpeed)))
  (if _ischecked
    (CallFunction|UpdateMovement (Variables|Movement|GetThrottleInput) (Variables|Movement|GetForwardForce))
    (CallFunction|UpdateRotation (Variables|Movement|GetTurnInput) (Variables|Movement|GetTurnTorque))))

(fn ConstructionScript)

(fn UpdateMovement
  (params (ThrottleInput :type Float%20%28double-precision%29) (ForwardForce :type Float%20%28double-precision%29))
  (bind _shipbody (Variables|Default|GetShipBody))
  (bind _returnvalue (Math|Vector|GetForwardVector _shipbody))
  (bind (_x _y) (Math|Vector|BreakVector _returnvalue))
  (if (> ThrottleInput 0.0)
    (Physics|AddForce (Variables|Default|GetShipBody) (* ForwardForce ThrottleInput (Class|KismetMathLibrary|VectorNormal2D (Math|Vector|MakeVector _x _y 0.0) 0.0001)) "None" true)))

(fn UpdateRotation
  (params (TurnInput :type Float%20%28double-precision%29) (TurnTorque :type Float%20%28double-precision%29))
  (Class|PrimitiveComponent|AddTorqueinDegrees (Variables|Default|GetShipBody) (* (Math|Vector|GetUpVector (Variables|Default|GetShipBody)) (* TurnInput TurnTorque)) "None" true))

(fn CannonRotation
  (params (IsAiming :type Boolean) (TurnYaw :type Float%20%28double-precision%29) (TurnPitch :type Float%20%28double-precision%29) (AimSensitivity :type Float%20%28double-precision%29))
  (bind _returnvalue (* AimSensitivity TurnPitch))
  (bind _returnvalue_2 (* TurnYaw AimSensitivity))
  (bind _returnvalue_3 (Math|Float|Clamp(Float) _returnvalue -7e+01 7e+01))
  (bind _returnvalue_4 (Math|Float|Clamp(Float) _returnvalue_2 -15.0 35.0))
  (if IsAiming
    (Transformation|SetRelativeRotation (Variables|Default|GetSpringArm) (Math|Rotator|MakeRotator 0.0 _returnvalue_3 _returnvalue_4) false false)
    (Transformation|SetRelativeRotation (Variables|Default|GetCannonYawPivot) (Math|Rotator|MakeRotator 0.0 0.0 _returnvalue_4) false false)
    (Transformation|SetRelativeRotation (Variables|Default|GetCannonPitchPivot) (Math|Rotator|MakeRotator 0.0 _returnvalue_3 0.0) false false)))

(fn MovementCheck
  (params (ThrottleInput :type Float%20%28double-precision%29) (MaxSpeed :type Float%20%28double-precision%29))
  (bind _returnvalue (Physics|GetPhysicsLinearVelocity (Variables|Default|GetShipBody) "None"))
  (return (and (> ThrottleInput 0.0) (< (Math|Vector|VectorLength (Math|Vector|MakeVector (.X (Math|Vector|BreakVector _returnvalue)) (.Y (Math|Vector|BreakVector _returnvalue)) 0.0)) MaxSpeed))))

(fn Fire
  (Game|SpawnActorfromClass "/Game/Blueprints/BP_CannonBall.BP_CannonBall_C" (Transformation|GetWorldTransform (Variables|Default|GetMuzzlePoint)) "Undefined" "MultiplyWithRoot" 0 0))