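; BP_Ship is a physics-driven ship with health, a spring-arm camera and a child-actor cannon exposed through GetMainCannon.
; Tick applies horizontal forward force and yaw torque as accelerations, both only while throttle is positive and horizontal speed is under MaxSpeed.
; TakeShipDamage clamps health, prints its fraction and destroys the ship at zero.
; IA_Aim is empty, leaving the aim and normal camera zoom logic unconnected.
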(event Custom|TakeShipDamage
  (params (DamageAmount :type Float%20%28double-precision%29))
  (bind _output_get (Variables|PlayerStatus|SetCurrentHealth (Math|Float|Clamp(Float) (- (Variables|PlayerStatus|GetCurrentHealth) DamageAmount) 0.0 (Variables|PlayerStatus|GetMaxHealth))))
  (bind _output_get_2 (Variables|PlayerStatus|SetHealthPercent (/ _output_get (Variables|PlayerStatus|GetMaxHealth))))
  (Development|PrintString (Utilities|String|ToString(Float) _output_get_2))
  (if (<= (Variables|PlayerStatus|GetCurrentHealth) 0.0)
    (Actor|DestroyActor)))

(event Input|EnhancedActionEvents|EnhancedInputActionIA_Aim
  (params (ActionValue :type Boolean) (ElapsedSeconds :type Float%20%28double-precision%29) (TriggeredSeconds :type Float%20%28double-precision%29) (InputAction :type Input%20Action%20Object%20Reference :default "/Game/Input/Action/IA_Aim.IA_Aim")))

(event EventBeginPlay
  (Variables|PlayerStatus|SetCurrentHealth (Variables|PlayerStatus|GetMaxHealth))
  (Variables|PlayerStatus|SetHealthPercent (/ (Variables|PlayerStatus|GetCurrentHealth) (Variables|PlayerStatus|GetMaxHealth))))

(event EventTick
  (params (DeltaSeconds :type Float%20%28single-precision%29))
  (bind _ischecked (CallFunction|MovementCheck (Variables|Movement|GetThrottleInput) (Variables|Movement|GetMaxSpeed)))
  (if _ischecked
    (CallFunction|UpdateMovement (Variables|Movement|GetThrottleInput) (Variables|Movement|GetForwardForce))
    (CallFunction|UpdateRotation (Variables|Movement|GetTurnInput) (Variables|Movement|GetTurnTorque))))

(fn ConstructionScript)

(fn UpdateMovement
  (params (ThrottleInput :type Float%20%28double-precision%29) (ForwardForce :type Float%20%28double-precision%29))
  (bind _shipbody (Variables|Default|GetShipBody))
  (bind _returnvalue (Math|Vector|GetForwardVector _shipbody))
  (bind (_x _y) (Math|Vector|BreakVector _returnvalue))
  (if (> ThrottleInput 0.0)
    (Physics|AddForce (Variables|Default|GetShipBody) (* ForwardForce ThrottleInput (Class|KismetMathLibrary|VectorNormal2D (Math|Vector|MakeVector _x _y 0.0) 0.0001)) "None" true)))

(fn UpdateRotation
  (params (TurnInput :type Float%20%28double-precision%29) (TurnTorque :type Float%20%28double-precision%29))
  (Class|PrimitiveComponent|AddTorqueinDegrees (Variables|Default|GetShipBody) (* (Math|Vector|GetUpVector (Variables|Default|GetShipBody)) (* TurnInput TurnTorque)) "None" true))

(fn MovementCheck
  (params (ThrottleInput :type Float%20%28double-precision%29) (MaxSpeed :type Float%20%28double-precision%29))
  (bind _returnvalue (Physics|GetPhysicsLinearVelocity (Variables|Default|GetShipBody) "None"))
  (return (and (> ThrottleInput 0.0) (< (Math|Vector|VectorLength (Math|Vector|MakeVector (.X (Math|Vector|BreakVector _returnvalue)) (.Y (Math|Vector|BreakVector _returnvalue)) 0.0)) MaxSpeed))))

(fn GetMainCannon
  (bind _asbp_cannon (Utilities|Casting|CastToBP_Cannon (Variables|/Script/Engine.ChildActorComponent|GetChildActor (Variables|Default|GetChildActor))))
  (return _asbp_cannon))