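; BP_Obstancle is a destructible obstacle actor that is destroyed when its health runs out.
; On BeginPlay it applies the MeshObstancle variable to its static mesh component, so the construction script leaves the mesh untouched.
; Incoming damage is subtracted from Health, clamped between zero and MaxHealth, and the actor destroys itself once Health reaches zero.
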(event Custom|TakeDamage
  (params (DamageAmount :type Integer))
  (Variables|Default|SetHealth (Math|Integer|Clamp(Integer) (- (Variables|Default|GetHealth) DamageAmount) 0 (Variables|Default|GetMaxHealth)))
  (if (<= (Variables|Default|GetHealth) 0)
    (Actor|DestroyActor)))

(event EventBeginPlay
  (Components|StaticMesh|SetStaticMesh (Variables|Default|GetStaticMesh) (Variables|Default|GetMeshObstancle)))

(event Collision|EventActorBeginOverlap
  (params (OtherActor :type Actor%20Object%20Reference)))

(event EventTick
  (params (DeltaSeconds :type Float%20%28single-precision%29)))

(fn ConstructionScript)