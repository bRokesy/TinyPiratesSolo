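; BP_Cannon is an aimable cannon that fires BP_CannonBall projectiles.
; AimCannon turns look input into frame-rate-scaled rotation, with free yaw on YawPivot and clamped pitch on PitchPivot.
; Fire spawns a cannonball at the Muzzle transform, gated by a cooldown checked against game time.
; Nothing in this Blueprint calls either function, so input has to come from outside.
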(event Collision|EventActorBeginOverlap
  (params (OtherActor :type Actor%20Object%20Reference)))

(event EventTick
  (params (DeltaSeconds :type Float%20%28single-precision%29)))

(fn ConstructionScript)

(fn AimCannon
  (params (LookX :type Float%20%28double-precision%29) (LookY :type Float%20%28double-precision%29))
  (Transformation|SetRelativeRotation (Variables|Default|GetYawPivot) (Math|Rotator|MakeRotator 0.0 0.0 (+ (* LookX (Variables|Default|GetYawSpeed) (Utilities|Time|GetWorldDeltaSeconds)) (.yaw (Variables|/Script/Engine.SceneComponent|GetRelativeRotation (Variables|Default|GetYawPivot))))) false false)
  (Transformation|SetRelativeRotation (Variables|Default|GetPitchPivot) (Math|Rotator|MakeRotator 0.0 (Math|Float|Clamp(Float) (- (.pitch (Variables|/Script/Engine.SceneComponent|GetRelativeRotation (Variables|Default|GetPitchPivot))) (* LookY (Utilities|Time|GetWorldDeltaSeconds) (Variables|Default|GetPitchSpeed))) (Variables|Default|GetMinPitch) (Variables|Default|GetMaxPitch)) 0.0) false false))

(fn Fire
  (if (>= (- (Utilities|Time|GetGameTimeinSeconds) (Variables|Default|GetLastFireTime)) (Variables|Default|GetFireCooldown))
    (Variables|Default|SetLastFireTime (Utilities|Time|GetGameTimeinSeconds))
    (Game|SpawnActorfromClass "/Game/Blueprints/BP_CannonBall.BP_CannonBall_C" (Transformation|GetWorldTransform (Variables|Default|GetMuzzle)) "Undefined" "MultiplyWithRoot" 0 0)))